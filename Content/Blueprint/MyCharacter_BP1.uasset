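; Player character Blueprint that handles input for UI menus, piece-based building and toolbar selection.
; Alt opens the build menu and enables Tick-driven BuildKit previews, with the mouse cycling, placing or cancelling pieces; Tab toggles inventory.
; Tick also swaps crosshair and HUD widgets on IsAR through cross-resetting DoOnce gates.
; Toolbar keys and left-click ammo use server calls; sprint logic is unwired, and BeginPlay calls DestroyActor on the owning controller.
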(event EventBeginPlay
  (bind _asplayer_controller (Utilities|Casting|CastToPlayerController (Pawn|GetController)))
  (Actor|DestroyActor (Game|Player|GetOwningPlayerController (Variables|/Script/Engine.PlayerController|GetPlayerCameraManager _asplayer_controller))))

(event EventTick
  (params (DeltaSeconds :type Float%20%28single-precision%29))
  (bind _returnvalue (Game|GetPlayerController 0))
  (bind _returnvalue_2 (Game|Player|GetPlayerPawn 0))
  (bind _asmy_character (Utilities|Casting|CastToMyCharacter _returnvalue_2))
  (if (Pawn|IsLocallyControlled _returnvalue_2)
    (Utilities|FlowControl|Sequence
      (:then_0
        (if (Variables|/Script/DeathVessels.MyCharacter|GetIsAR _asmy_character)
          (Utilities|FlowControl|DoOnce false :!label _label
            (:Completed
              (Viewport|RemoveAllWidgets)
              (bind _returnvalue_3 (UserInterface|CreateWidget "/Game/Widgets/Crosshair.Crosshair_C" _returnvalue))
              (UserInterface|Viewport|AddtoViewport _returnvalue_3 0)
              (Variables|Default|SetUI%20Switched true)
              (Input|SetInputModeGameOnly _returnvalue)
              (goto _label_2 Reset)))
          (else
            (if (Variables|Default|GetUI%20Switched)
              (Viewport|RemoveAllWidgets))
            (Utilities|FlowControl|DoOnce false :!label _label_2
              (:Completed
                (bind _returnvalue_4 (UserInterface|CreateWidget "/Game/Widgets/HUD.HUD_C" _returnvalue))
                (UserInterface|Viewport|AddtoViewport _returnvalue_4 0)
                (Variables|Default|SetUI%20Switched false)
                (goto _label Reset))))))
      (:then_1
        (if (Variables|Default|GetAllowBuild)
          (bind _exitbuildingpiece (Class|MyCharacter|BuildKit (Variables|Default|GetBuilding%20Piece)))
          (Variables|Default|SetBuilding%20Piece _exitbuildingpiece))))))

(event Input|KeyboardEvents|LeftAlt
  (params (Key :type Key%20Structure :default "None"))
  (bind _returnvalue (Game|GetPlayerController 0))
  (:Pressed
    (Viewport|RemoveAllWidgets)
    (bind _returnvalue_2 (UserInterface|CreateWidget "/Game/Widgets/buildmenu.buildmenu_C" _returnvalue))
    (Variables|/Script/Engine.PlayerController|SetbShowMouseCursor _returnvalue true)
    (Input|SetInputModeGameandUI _returnvalue 0 "LockOnCapture" true)
    (UserInterface|Viewport|AddtoViewport _returnvalue_2 0)
    (Variables|Default|SetAllowBuild true)))

(event Input|KeyboardEvents|Tab
  (params (Key :type Key%20Structure :default "None"))
  (bind _returnvalue (Game|GetPlayerController 0))
  (:Pressed
    (Utilities|FlowControl|FlipFlop
      (:A
        (Viewport|RemoveAllWidgets)
        (bind _returnvalue_2 (UserInterface|CreateWidget "/Game/Widgets/Inventory_UI.Inventory_UI_C" _returnvalue))
        (Variables|/Script/Engine.PlayerController|SetbShowMouseCursor _returnvalue true)
        (Input|SetInputModeGameandUI _returnvalue 0 "LockOnCapture" true)
        (UserInterface|Viewport|AddtoViewport _returnvalue_2 0))
      (:B
        (Viewport|RemoveAllWidgets)
        (Variables|/Script/Engine.PlayerController|SetbShowMouseCursor _returnvalue false)
        (Input|SetInputModeGameOnly _returnvalue)))))

(event Input|KeyboardEvents|5
  (params (Key :type Key%20Structure :default "None"))
  (:Pressed
    (Class|MyCharacter|ServerPlayerToolbar Key (Variables|Default|GetItemName))))

(event Input|MouseEvents|MouseWheelUp
  (params (Key :type Key%20Structure :default "None"))
  (:Pressed
    (bind _returnvalue (Class|MyCharacter|SwitchUp (Variables|Default|GetBuilding%20Piece)))
    (Variables|Default|SetBuilding%20Piece _returnvalue)))

(event Input|MouseEvents|MouseWheelDown
  (params (Key :type Key%20Structure :default "None"))
  (:Pressed
    (bind _returnvalue (Class|MyCharacter|SwitchDown (Variables|Default|GetBuilding%20Piece)))
    (Variables|Default|SetBuilding%20Piece _returnvalue)))

(event Input|MouseEvents|RightMouseButton
  (params (Key :type Key%20Structure :default "None"))
  (:Pressed
    (Class|MyCharacter|CleanupBuild)))

(event Input|MouseEvents|LeftMouseButton
  (params (Key :type Key%20Structure :default "None"))
  (bind _ishatchet (Variables|Default|GetIsHatchet))
  (bind _returnvalue (Math|Boolean|Equal(Boolean) _ishatchet false))
  (:Pressed
    (Utilities|FlowControl|Sequence
      (:then_0
        (if (and (Math|Boolean|Equal(Boolean) (Variables|Default|GetIsAR) false) _returnvalue)
          (Class|MyCharacter|FindPlacementLocation (Variables|Default|GetBuilding%20Piece))))
      (:then_1
        (if _returnvalue
          (bind _asmy_character (Utilities|Casting|CastToMyCharacter (Game|Player|GetPlayerPawn 0)))
          (Class|InventoryTest|ServerAddAmmo (Variables|/Script/DeathVessels.MyCharacter|GetInventoryTest _asmy_character)))))))

(event Input|KeyboardEvents|1
  (params (Key :type Key%20Structure :default "None"))
  (:Pressed
    (Class|MyCharacter|ServerPlayerToolbar Key (Variables|Default|GetItemName))))

(event Input|KeyboardEvents|2
  (params (Key :type Key%20Structure :default "None"))
  (:Pressed
    (Class|MyCharacter|ServerPlayerToolbar Key (Variables|Default|GetItemName))))

(event Input|KeyboardEvents|3
  (params (Key :type Key%20Structure :default "None"))
  (:Pressed
    (Class|MyCharacter|ServerPlayerToolbar Key (Variables|Default|GetItemName))))

(event Input|KeyboardEvents|4
  (params (Key :type Key%20Structure :default "None"))
  (:Pressed
    (Class|MyCharacter|ServerPlayerToolbar Key (Variables|Default|GetItemName))))

(fn ConstructionScript)